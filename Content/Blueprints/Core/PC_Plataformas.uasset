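; PC_Plataformas is the player controller for a platformer level and owns the HUD.
; On BeginPlay it creates and shows WBP_HUD, then resets the stats in GI_Plataformas.
; Its UI events forward health and collected/total item counts to the HUD widget, with the health update intended to be called from the GameInstance.
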(event Custom|ActualizarVidaEnUI
  (params (Vida :type Float%20%28double-precision%29))
  ;[0.15 0.15 0.15 0.5] Recibe llamada del GameInstance y actualiza vida
  (Default|ActualizarVida (Variables|Default|GetHUDWidget) Vida))

(event Custom|ActualizarItemsEnUI
  (params (Recolectados :type Integer) (Totales :type Integer))
  ;[0.15 0.15 0.15 0.5] Comentario
  (Default|ActualizarItems (Variables|Default|GetHUDWidget) Recolectados Totales))

(event EventBeginPlay
  ;[0.15 0.15 0.15 0.5] Crear y mostrar el HUD al inicio del nivel
  (Development|PrintString "PC: BeginPlay disparado")
  (bind _returnvalue (UserInterface|CreateWidget "/Game/UI/WBP_HUD.WBP_HUD_C"))
  (bind _output_get (Variables|Default|SetHUDWidget _returnvalue))
  (UserInterface|Viewport|AddtoViewport _output_get 0)
  (bind _asgi_plataformas (Utilities|Casting|CastToGI_Plataformas (Game|GetGameInstance)))
  (Default|ResetearStats _asgi_plataformas))

(fn ConstructionScript)