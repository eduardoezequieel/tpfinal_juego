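; GI_Plataformas, apparently the platformer's Game Instance, tracks player health, collected items and the win state.
; ModificarVida adds to health, caps it at the maximum and opens Lvl_ThirdPerson by name when it reaches zero or below.
; ModificarItems adds to the collected count and sets Gano once the total is reached.
; ResetearStats restores health, item count and win flag, but the death branch does not call it.
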(event Custom|ModificarVida
  (params (Valor :type Float%20%28double-precision%29))
  ;[0.15 0.15 0.15 0.5] Suma valor a vida actual
  (bind _output_get (Variables|Default|SetVida (+ Valor (Variables|Default|GetVida))))
  ;[0.15 0.15 0.15 0.5] Vida no puede superar vida máxima
  (if (> _output_get (Variables|Default|GetVidaMaxima))
    (Variables|Default|SetVida (Variables|Default|GetVidaMaxima)))
  ;[0.15 0.15 0.15 0.5] Si vida es menor o igual que cero, reiniciar nivel
  (if (<= (Variables|Default|GetVida) 0.0)
    (Game|OpenLevel(byName) "Lvl_ThirdPerson")))

(event Custom|ModificarItems
  (params (Cantidad :type Integer))
  ;[0.15 0.15 0.15 0.5] Suma items y verifica victoria
  (bind _output_get (Variables|Default|SetItemsRecolectados (+ Cantidad (Variables|Default|GetItemsRecolectados))))
  (if (>= _output_get (Variables|Default|GetItemsTotales))
    (Variables|Default|SetGano true)))

(event Custom|ResetearStats
  ;[0.15 0.15 0.15 0.5] Reiniciar juego
  (Variables|Default|SetVida 1e+02)
  (Variables|Default|SetItemsRecolectados 0)
  (Variables|Default|SetGano false))